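; Tower defense transistor tower that tracks virus actors inside its range and turns to aim at them; no firing logic is present.
; Range overlaps maintain a target list, from which a random target is picked when none is active or the current one leaves.
; A gated, per-frame Delay loop splits aiming into Sphere yaw and Cylinder pitch in actor-local space.
; Without a target it enters a rest-reset branch, whose cancel and continue events are empty.
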(event OnComponentBeginOverlap(towerRange)
  (params (OverlappedComponent :type Primitive%20Component%20Object%20Reference) (OtherActor :type Actor%20Object%20Reference) (OtherComp :type Primitive%20Component%20Object%20Reference) (OtherBodyIndex :type Integer) (bFromSweep :type Boolean) (SweepResult :type Hit%20Result%20Structure%20%28by%20ref%29))
  ;[1 1 1] overlap detection
  (bind _asvirus (Utilities|Casting|CastTovirus OtherActor))
  (Utilities|Array|Add (Variables|Default|GetTargetsInRange) _asvirus)
  (Utilities|IsValid (Variables|Default|GetTarget)
    (:Is%20Not%20Valid
      (CallFunction|SelectTarget))))

(event OnComponentEndOverlap(towerRange)
  (params (OverlappedComponent :type Primitive%20Component%20Object%20Reference) (OtherActor :type Actor%20Object%20Reference) (OtherComp :type Primitive%20Component%20Object%20Reference) (OtherBodyIndex :type Integer))
  (bind _targetsinrange (Variables|Default|GetTargetsInRange))
  ;[1 1 1] overlap detection
  (bind _asvirus (Utilities|Casting|CastTovirus OtherActor))
  (if (Utilities|Array|ContainsItem _targetsinrange 0)
    (Utilities|Array|RemoveItem _targetsinrange 0)
    (if (== _asvirus (Variables|Default|GetTarget))
      (Variables|Default|SetTarget 0)
      (CallFunction|SelectTarget))))

(event Custom|SelectTarget
  (bind _targetsinrange (Variables|Default|GetTargetsInRange))
  (if (Utilities|Array|IsValidIndex _targetsinrange)
    (Variables|Default|SetTarget (Utilities|Array|Get(acopy) _targetsinrange (Math|Random|RandomIntegerinRange 0 (Utilities|Array|LastIndex _targetsinrange))))
    (CallFunction|BeginAim)
    (else
      (CallFunction|BeginRest))))

(event Custom|BeginAim
  (bind _cylinder (Variables|Default|GetCylinder))
  (bind _returnvalue (Transformation|GetWorldLocation _cylinder))
  (Utilities|FlowControl|Sequence
    (:then_0
      (goto _label Open))
    (:then_1
      (Utilities|FlowControl|Gate true :!label _label
        (:Exit
          (Utilities|IsValid (Variables|Default|GetTarget)
            (:Is%20Valid
              (Variables|Default|SetTargetLocation (Transformation|GetActorLocation (Variables|Default|GetTarget)))
              (Transformation|SetRelativeRotation (Variables|Default|GetSphere) (Math|Rotator|MakeRotator 0.0 0.0 (.Yaw (Math|Rotator|BreakRotator (Math|Rotator|MakeRotfromX (Math|Transform|InverseTransformDirection (Transformation|GetActorTransform) (Math|Vector|MakeVector (- (.x (Variables|Default|GetTargetLocation)) (.x _returnvalue)) (- (.y (Variables|Default|GetTargetLocation)) (.y _returnvalue)) (- (.z (Variables|Default|GetTargetLocation)) (.z _returnvalue)))))))) false false)
              (Transformation|SetRelativeRotation (Variables|Default|GetCylinder) (Math|Rotator|MakeRotator 0.0 (.Pitch (Math|Rotator|BreakRotator (Math|Rotator|MakeRotfromX (Math|Transform|InverseTransformDirection (Transformation|GetActorTransform) (Math|Vector|MakeVector (- (.x (Variables|Default|GetTargetLocation)) (.x _returnvalue)) (- (.y (Variables|Default|GetTargetLocation)) (.y _returnvalue)) (- (.z (Variables|Default|GetTargetLocation)) (.z _returnvalue))))))) 0.0) false false)
              (Utilities|FlowControl|Delay (Utilities|Time|GetWorldDeltaSeconds))
              (CallFunction|ContinueAim))
            (:Is%20Not%20Valid
              (CallFunction|CancelAim)
              (CallFunction|BeginRest))))))))

(event Custom|BeginRest
  (bind _returnvalue (Math|Rotator|MakeRotator 0.0 0.0 0.0))
  (bind _returnvalue_2 (Math|Rotator|MakeRotator 0.0 0.0 0.0))
  (Utilities|FlowControl|Sequence
    (:then_0
      (goto _label Open))
    (:then_1
      (Utilities|FlowControl|Gate true :!label _label
        (:Exit
          (Utilities|IsValid (Variables|Default|GetTarget)
            (:Is%20Valid
              (CallFunction|CancelReset :!label _label_2))
            (:Is%20Not%20Valid
              (if (and (Utilities|Operators|EqualEqual :A _returnvalue_2) (Utilities|Operators|EqualEqual :A _returnvalue))
                (goto _label_2)
                (else
                  (Transformation|SetRelativeRotation _returnvalue_2 false false)
                  (Transformation|SetRelativeRotation _returnvalue false false))))))))))

(event Custom|CancelAim
  (bind _cylinder (Variables|Default|GetCylinder))
  (bind _returnvalue (Transformation|GetWorldLocation _cylinder))
  (Utilities|FlowControl|Gate true) ; enters at Close
)

(event Custom|ContinueAim
  (bind _cylinder (Variables|Default|GetCylinder))
  (bind _returnvalue (Transformation|GetWorldLocation _cylinder))
  (Utilities|IsValid (Variables|Default|GetTarget)
    (:Is%20Valid
      (Utilities|FlowControl|Gate true
        (:Exit
          (Utilities|IsValid (Variables|Default|GetTarget)
            (:Is%20Valid
              (Variables|Default|SetTargetLocation (Transformation|GetActorLocation (Variables|Default|GetTarget)))
              (Transformation|SetRelativeRotation (Variables|Default|GetSphere) (Math|Rotator|MakeRotator 0.0 0.0 (.Yaw (Math|Rotator|BreakRotator (Math|Rotator|MakeRotfromX (Math|Transform|InverseTransformDirection (Transformation|GetActorTransform) (Math|Vector|MakeVector (- (.x (Variables|Default|GetTargetLocation)) (.x _returnvalue)) (- (.y (Variables|Default|GetTargetLocation)) (.y _returnvalue)) (- (.z (Variables|Default|GetTargetLocation)) (.z _returnvalue)))))))) false false)
              (Transformation|SetRelativeRotation (Variables|Default|GetCylinder) (Math|Rotator|MakeRotator 0.0 (.Pitch (Math|Rotator|BreakRotator (Math|Rotator|MakeRotfromX (Math|Transform|InverseTransformDirection (Transformation|GetActorTransform) (Math|Vector|MakeVector (- (.x (Variables|Default|GetTargetLocation)) (.x _returnvalue)) (- (.y (Variables|Default|GetTargetLocation)) (.y _returnvalue)) (- (.z (Variables|Default|GetTargetLocation)) (.z _returnvalue))))))) 0.0) false false)
              (Utilities|FlowControl|Delay (Utilities|Time|GetWorldDeltaSeconds))
              (CallFunction|ContinueAim))
            (:Is%20Not%20Valid
              (CallFunction|CancelAim :!label _label)
              (CallFunction|BeginRest))))))
    (:Is%20Not%20Valid
      (goto _label))))

(event Custom|CancelReset)

(event Custom|ContinueReset)

(fn ConstructionScript)