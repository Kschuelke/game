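; Virus enemy that walks to an Endpoint actor and damages the CPU when it gets there.
; The spawnmove event runs AI MoveTo, and on success applies damage once to the first BP_CPU found, then destroys the virus.
; BeginPlay seeds the health bar widget with MaxHealth.
; AnyDamage subtracts from Health, updates the bar and destroys the virus at zero or below.
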(event Custom|spawnmove
  (AI|AIMoveTo self "0, 0, 0" (Variables|Default|GetEndpoint) 5.0 false
    (:OnSuccess
      (Utilities|FlowControl|DoOnce false
        (:Completed
          (bind _outactors (Actor|GetAllActorsOfClass "/Game/Blueprints/BP_CPU.BP_CPU_C"))
          (Game|Damage|ApplyDamage (Utilities|Array|Get(acopy) _outactors) 1.0 0 self)
          (Actor|DestroyActor))))))

(event Game|Damage|EventAnyDamage
  (params (Damage :type Float%20%28single-precision%29) (DamageType :type Damage%20Type%20Object%20Reference) (InstigatedBy :type Controller%20Object%20Reference) (DamageCauser :type Actor%20Object%20Reference))
  ;[1 1 1] Recieve Damage
  (bind _output_get (Variables|Default|SetHealth (- (Variables|Default|GetHealth) Damage)))
  (Variables|/Game/Blueprints/EnemeHealthBarBP.EnemeHealthBarBP_C|SetHealth (Variables|Default|GetEneme%20Health%20Bar%20Ref) _output_get)
  (if (<= (Variables|Default|GetHealth) 0.0)
    (Utilities|FlowControl|DoOnce false
      (:Completed
        (Actor|DestroyActor)))))

(event EventBeginPlay
  ;[1 1 1] Comment
  (bind _aseneme_health_bar_bp (Utilities|Casting|CastToEnemeHealthBarBP (UserInterface|GetUserWidgetObject (Variables|Default|GetHealthBar))))
  (bind _output_get (Variables|Default|SetEneme%20Health%20Bar%20Ref _aseneme_health_bar_bp))
  (Variables|/Game/Blueprints/EnemeHealthBarBP.EnemeHealthBarBP_C|SetMaxHealth _output_get (Variables|Default|GetMaxHealth))
  (Variables|/Game/Blueprints/EnemeHealthBarBP.EnemeHealthBarBP_C|SetHealth _output_get (Variables|Default|GetMaxHealth)))

(fn ConstructionScript)