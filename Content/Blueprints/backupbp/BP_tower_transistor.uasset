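; Transistor tower Blueprint that turns to aim at Virus actors within range; it contains no firing logic.
; Each tick it takes the first Virus found in the level, not the nearest, and checks its distance against a fixed radius.
; AimAtTarget converts the direction to the target into actor-local space, applying yaw to the Sphere and pitch to the Cylinder.
; ResetAim is called when that Virus is out of range but is empty.
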(event Custom|aim%20at%20target
  (bind _returnvalue (Transformation|GetActorTransform))
  (bind _targetlocation (Variables|Default|GetTargetLocation))
  (bind _cylinder (Variables|Default|GetCylinder))
  (bind _returnvalue_2 (Transformation|GetWorldLocation _cylinder))
  (bind _returnvalue_3 (- (.x _targetlocation) (.x _returnvalue_2)))
  (bind _returnvalue_4 (- (.y _targetlocation) (.y _returnvalue_2)))
  (bind _returnvalue_5 (- (.z _targetlocation) (.z _returnvalue_2)))
  (bind _returnvalue_6 (Math|Vector|MakeVector _returnvalue_3 _returnvalue_4 _returnvalue_5))
  (bind _returnvalue_7 (Math|Transform|InverseTransformDirection _returnvalue _returnvalue_6))
  (bind _returnvalue_8 (Math|Rotator|MakeRotfromX _returnvalue_7))
  (Transformation|SetRelativeRotation (Variables|Default|GetSphere) (Math|Rotator|MakeRotator 0.0 0.0 (.Yaw (Math|Rotator|BreakRotator _returnvalue_8))) false false)
  (Transformation|SetRelativeRotation (Variables|Default|GetCylinder) (Math|Rotator|MakeRotator 0.0 (.Pitch (Math|Rotator|BreakRotator _returnvalue_8)) 0.0) false false))

(event Custom|reset%20aim)

(event EventTick
  (params (DeltaSeconds :type Float%20%28single-precision%29))
  (bind _returnvalue (Transformation|GetActorLocation))
  (bind _outactors (Actor|GetAllActorsOfClass "/Game/Blueprints/virus.virus_C"))
  (if (Utilities|Array|IsValidIndex _outactors)
    (Variables|Default|SetTarget (Utilities|Array|Get(acopy) _outactors))
    ;[1 1 1] Get target location
    (Variables|Default|SetTargetLocation (Transformation|GetActorLocation (Variables|Default|GetTarget)))
    ;[1 1 1] check target distance
    (if (<= (Math|Vector|VectorLength (Math|Vector|MakeVector (- (.x _returnvalue) (.x (Variables|Default|GetTargetLocation))) (- (.y _returnvalue) (.y (Variables|Default|GetTargetLocation))) (- (.z _returnvalue) (.z (Variables|Default|GetTargetLocation))))) 2e+03)
      (CallFunction|AimatTarget)
      (else
        (CallFunction|ResetAim)))))

(fn ConstructionScript)