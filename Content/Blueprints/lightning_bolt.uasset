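; Lightning bolt projectile actor that damages virus actors it touches.
; It records its start location on BeginPlay and checks distance each Tick, destroying itself once it reaches ProjectileRange.
; A StaticMesh overlap casts the other actor to virus, applies Damage, then destroys the bolt, ignoring other actor types.
; Separate DoOnce nodes make the range expiry and the hit each fire only once.
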(event OnComponentBeginOverlap(StaticMesh)
  (params (OverlappedComponent :type Primitive%20Component%20Object%20Reference) (OtherActor :type Actor%20Object%20Reference) (OtherComp :type Primitive%20Component%20Object%20Reference) (OtherBodyIndex :type Integer) (bFromSweep :type Boolean) (SweepResult :type Hit%20Result%20Structure%20%28by%20ref%29))
  (bind _asvirus (Utilities|Casting|CastTovirus OtherActor))
  (Utilities|FlowControl|DoOnce false
    (:Completed
      (Game|Damage|ApplyDamage _asvirus (Variables|Default|GetDamage) 0 self)
      (Actor|DestroyActor))))

(event EventBeginPlay
  (Variables|Default|SetStartLocation (Transformation|GetActorLocation)))

(event EventTick
  (params (DeltaSeconds :type Float%20%28single-precision%29))
  ;[1 1 1] distance it can travel before destroying itself
  (if (>= (Math|Vector|VectorLength (- (Variables|Default|GetStartLocation) (Transformation|GetActorLocation))) (Variables|Default|GetProjectileRange))
    (Utilities|FlowControl|DoOnce false
      (:Completed
        (Actor|DestroyActor)))))

(fn ConstructionScript)